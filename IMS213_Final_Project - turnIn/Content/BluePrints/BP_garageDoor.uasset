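; Garage door actor that starts locked with a red status light and raises or lowers when the third-person character overlaps it.
; EventUnlockDoor clears the lock and turns the light green after a short delay.
; State flags gate each overlap toggle, and two timelines offset the door's height from its starting position.
; LowerDoor's completion is unwired, so the door stays flagged as moving after lowering and ignores further overlaps.
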(event Custom|EventUnlockDoor
  ;[1 1 1] unlock door and change indicator color
  (Variables|Default|SetdoorIsLocked false)
  (Utilities|FlowControl|Delay 0.75)
  (Rendering|Material|SetMaterial (Variables|Default|GetstatusLight) 0 "/Game/Assets/MM_statusGreen.MM_statusGreen"))

(event Custom|eventRaiseDoor
  ;[1 1 1] raise the door
  (Variables|Default|SetdoorIsDown false)
  (bind _garagedoorheight (Timeline|raise%20the%20door PlayFromStart)
    (:Update
      (Transformation|SetWorldLocation (Variables|Default|Getdoor) (Math|Vector|MakeVector (Variables|Default|GetstartX) (Variables|Default|GetstartY) (+ _garagedoorheight (Variables|Default|GetstartZ))) false false))
    (:Finished
      (Variables|Default|SetdoorIsUp true)
      (Variables|Default|SetdoorIsMoving false))))

(event Custom|eventLowerDoor
  ;[1 1 1] lower door
  (Variables|Default|SetdoorIsUp false)
  (bind _garage_door_height (Timeline|lower%20door PlayFromStart)
    (:Update
      (Transformation|SetWorldLocation (Variables|Default|Getdoor) (Math|Vector|MakeVector (Variables|Default|GetstartX) (Variables|Default|GetstartY) (+ _garage_door_height (Variables|Default|GetstartZ))) false false))))

(event EventBeginPlay
  (bind _door (Variables|Default|Getdoor))
  (bind _returnvalue (Transformation|GetWorldLocation _door))
  ;[1 1 1] initialize the variables
  (Variables|Default|SetstartX (.x _returnvalue))
  (Variables|Default|SetstartY (.y _returnvalue))
  (Variables|Default|SetstartZ (.z _returnvalue))
  (Variables|Default|SetdoorIsDown true)
  (Variables|Default|SetdoorIsUp false)
  (Variables|Default|SetdoorIsMoving false)
  (Variables|Default|SetdoorIsLocked true)
  (Rendering|Material|SetMaterial (Variables|Default|GetstatusLight) 0 "/Game/Assets/MM_statusRed.MM_statusRed"))

(event Collision|EventActorBeginOverlap
  (params (OtherActor :type Actor%20Object%20Reference))
  ;[1 1 1] raise and lower door
  (Utilities|Casting|CastToBP_ThirdPersonCharacter OtherActor)
  (if (not (Variables|Default|GetdoorIsLocked))
    (if (not (Variables|Default|GetdoorIsMoving))
      (if (Variables|Default|GetdoorIsUp)
        (Variables|Default|SetdoorIsMoving true)
        (CallFunction|EventLowerDoor)
        (elif (Variables|Default|GetdoorIsDown)
          (Variables|Default|SetdoorIsMoving true)
          (CallFunction|EventRaiseDoor))))))

(fn ConstructionScript)